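; Crow City citizen NPC that picks random destinations, walks waypoint paths and searches for post collection boxes.
; State-driven events move it from Idle to Goto, fetch a destination from DM and issue AI moves through PathToFollow via its controller.
; FindPCBox widens a sphere trace across calls until it finds a box, then ignores that box once within range.
; Tick optionally draws the active path for debugging.
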(event `self.ReceiveTick`
  (params (DeltaSeconds :type "Float (single-precision)"))
  (bind _pathtofollow (`self.PathToFollow`))
  (bind _pathtofollow_2 (`self.PathToFollow`))
  (bind _pathtofollow_3 (`self.PathToFollow`))
  (bind _returnvalue (- (`KismetArrayLibrary.Array_Length` _pathtofollow_2) 1))
  (`parent.ReceiveTick` DeltaSeconds)
  (if (and (`self.ShowDebug`) (`self.IsNavigating`))
    (`KismetSystemLibrary.DrawDebugSphere` (`|GetArrayItem` _pathtofollow_2) 100.0 12 (struct :`G` 0.246284 :`B` 1.0 :`A` 1.0) 0.1 2.0)
    (`KismetSystemLibrary.DrawDebugSphere` (`|GetArrayItem` _pathtofollow_2 _returnvalue) 100.0 12 (struct :`G` 1.0 :`B` 0.574655 :`A` 1.0) 0.1 2.0)
    (for _index (range 1 _returnvalue)
      (`KismetSystemLibrary.DrawDebugSphere` (`|GetArrayItem` _pathtofollow _index) 100.0 12 (struct :`R` 1.0 :`G` 0.316846 :`A` 1.0) 0.1 2.0)
      (for (_array_element _array_index) _pathtofollow
        (if (< _array_index (- (`KismetArrayLibrary.Array_Length` _pathtofollow_3) 1))
          (`KismetSystemLibrary.DrawDebugLine` _array_element (`|GetArrayItem` _pathtofollow_3 (+ _array_index 1)) (struct :`R` 1.0 :`B` 0.17413 :`A` 1.0) 1.0 10.0))))))

(event `MoveOnPath`
  (bind _pathtofollow (`self.PathToFollow`))
  (bind _pathindex (`self.PathIndex`))
  ;[1 1 1] MoveOnPath
  (if (< _pathindex (`KismetArrayLibrary.Array_Length` _pathtofollow))
    (set `self.IsNavigating` true)
    (bind _ascrow_city_citizen_controller_bp (cast `/Game/AI/CrowCityCitizenController_BP` (`self.GetController`)))
    (`AITask_MoveTo.AIMoveTo` _ascrow_city_citizen_controller_bp (`|GetArrayItem` _pathtofollow _pathindex) null
      (:`then`
        (`/Engine/EditorBlueprintResources/StandardMacros.IncrementInt` (`self.PathIndex`))))
    (else
      (set `self.IsNavigating` false)
      (`self.SetNPCState` "Idle"))))

(event `self.PickWorkToDo`
  (if (`|EnumEquality` (`self.NPCState`) "Idle")
    (`self.SetNPCState` "Goto")
    (`KismetSystemLibrary.PrintString` "CC")))

(event `self.FindDestinationToMove`
  (bind _dm (`self.DM`))
  (if (`|EnumEquality` (`self.NPCState`) "Goto")
    (`/Engine/EditorBlueprintResources/StandardMacros.IsValid` _dm
      (:`Is Valid`
        (set `self.CurrentDestination` (`Destination.DestinationLocaton` (`DestinationManager.GetRandomDestination` _dm)))
        (set `self.bHasDestinationToMove` true))
      (:`Is Not Valid`
        (set `self.bHasDestinationToMove` false :!label _label)
        (`self.SetNPCState` "Idle")))
    (else
      (goto _label))))

(fn `FindPCBox`
  (bind _returnvalue (`self.K2_GetActorLocation`))
  (`/Engine/EditorBlueprintResources/StandardMacros.IsValid` (`self.TargetBox`)
    (:`Is Valid`
      (if (< (`KismetMathLibrary.VSize` (- (`self.K2_GetActorLocation` (`self.TargetBox`)) (`self.K2_GetActorLocation`))) 300.0)
        (`KismetArrayLibrary.Array_Add` (`self.IgnoreActors`) (`self.TargetBox`))
        (set `self.TargetBox` null)))
    (:`Is Not Valid`
      (bind _output_get (set `self.Traceradius` (+ (`self.Traceradius`) 5.0)))
      (if (> _output_get (.x (`.BoxExtent` (`self.GetActorBounds` (`self.LevelNavMesh`) false false))))
        (set `self.Traceradius` 0.0))
      (bind _outhit (`KismetSystemLibrary.SphereTraceSingleForObjects` _returnvalue (+ _returnvalue (1.0 0.0 0.0)) (`self.Traceradius`) (`|MakeArray` "ObjectTypeQuery7" :!type "EObjectTypeQuery Enum") true (`self.IgnoreActors`) "ForOneFrame"))
      (bind _aspost_collecton_bp (cast `/Game/Blueprints/PostCollecton_BP` (`.HitActor` (`GameplayStatics.BreakHitResult` _outhit))))
      (set `self.TargetBox` _aspost_collecton_bp)
      (set `self.Traceradius` 0.0))))

(fn `UserConstructionScript`
  (`parent.UserConstructionScript`)
  (bind _returnvalue (`GameplayStatics.GetActorOfClass` "/Script/NavigationSystem.NavMeshBoundsVolume"))
  (`/Engine/EditorBlueprintResources/StandardMacros.IsValid` _returnvalue
    (:`Is Valid`
      (set `self.LevelNavMesh` _returnvalue))))