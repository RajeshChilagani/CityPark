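; Base destination building actor for AI, representing a school, office, hospital or stadium according to its DestinationType.
; The construction script switches on the type to set the mesh's material and write the building name to the Name text component.
; On BeginPlay it stores the Door component's world location as the destination location.
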(event `self.ReceiveBeginPlay`
  (set `self.DestinationLocaton` (`SceneComponent.K2_GetComponentLocation` (`self.Door`))))

(fn `UserConstructionScript`
  (bind _mesh (`self.Mesh`))
  (switch `EDestinationType` (`self.destinationType`)
    (:`School`
      (`PrimitiveComponent.SetMaterial` _mesh 0 "/Game/Materials/MI_Schools.MI_Schools")
      (set `self.Building Name` "SCHOOL"))
    (:`Office`
      (`PrimitiveComponent.SetMaterial` _mesh 0 "/Game/Materials/MI_Offices.MI_Offices")
      (set `self.Building Name` "OFFICE"))
    (:`Hospital`
      (`PrimitiveComponent.SetMaterial` _mesh 0 "/Game/Materials/MI_Hospitals.MI_Hospitals")
      (set `self.Building Name` "HOSPITAL"))
    (:`Stadium`
      (`PrimitiveComponent.SetMaterial` _mesh 0 "/Game/Materials/MI_Stadiums.MI_Stadiums")
      (set `self.Building Name` "STADIUM")))
  (`TextRenderComponent.K2_SetText` (`self.Name`) (`self.Building Name`)))