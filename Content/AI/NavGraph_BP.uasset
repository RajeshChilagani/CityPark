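; Navigation graph actor that spawns attached NavPoint_BP nodes and finds paths between world positions across them.
; FindPathToTarget snaps source and destination to nav points, calls GeneratePathInPositions, then appends the exact destination to any non-empty path; its UseAStar input is unused.
; Nearest-point lookup repeats a sphere trace, growing the shared TraceRadius until a hit.
; The construction script can enable debug on all nav points; path-drawing test code is disconnected.
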(event `self.ReceiveBeginPlay`)

(event `self.ReceiveTick`
  (params (DeltaSeconds :type "Float (single-precision)")))

(fn `CreateNavPoint`
  (bind _returnvalue (`|SpawnActorFromClass` "/Game/AI/NavPoint_BP.NavPoint_BP_C" (`self.GetTransform`) "AlwaysSpawn" "OverrideRootScale" self null))
  (`self.K2_AttachToActor` _returnvalue self "None" "KeepWorld" "KeepRelative" "KeepRelative" true))

(fn `Find Closest Nav Point`
  (params (Location :type "Vector Structure"))
  (returns (NP :type "NavPoint Object Reference"))
  (locals (TraceRadius :type "Float (double-precision)" :default 1.0))
  (while true
    (bind (_outhit _returnvalue) (`KismetSystemLibrary.SphereTraceSingleForObjects` :`Start` Location :`End` (+ Location (1.0 0.0 0.0)) :`Radius` (`local.TraceRadius`) :`ObjectTypes` (`|MakeArray` "ObjectTypeQuery8" :!type "EObjectTypeQuery Enum") :`DrawDebugType` "ForOneFrame" :`DrawTime` 1.0))
    (if _returnvalue
      (bind _asnav_point (cast `NavPoint` (`.HitActor` (`GameplayStatics.BreakHitResult` _outhit))))
      (return _asnav_point)
      (else
        (set `local.TraceRadius` (+ (`local.TraceRadius`) 0.5))))))

(fn `FindPathToTarget`
  (params (Source :type "Vector Structure") (Destination :type "Vector Structure") (UseAStar :type Boolean :default false))
  (returns (PathOut :type "Array of Vector Structure"))
  (`|ExecutionSequence`
    (:`then_0`
      (bind _np (`self.Find Closest Nav Point` Source))
      (set `self.SourceNavPoint` _np)
      (bind _np_2 (`self.Find Closest Nav Point` Destination))
      (set `self.DestNavPoint` _np_2)
      (`KismetArrayLibrary.Array_Clear` (`self.Path`)))
    (:`then_1`
      (bind _returnvalue (`self.GeneratePathInPositions` (`self.SourceNavPoint`) (`self.DestNavPoint`)))
      (bind _output_get (set `self.Path` _returnvalue))
      (`|ExecutionSequence`
        (:`then_0`
          (if (> (`KismetArrayLibrary.Array_Length` _output_get) 0)
            (`KismetArrayLibrary.Array_Add` (`self.Path`) Destination)))
        (:`then_1`
          (return (`self.Path`)))))))

(fn `UserConstructionScript`
  (if (`self.bShowDebug`)
    (bind _outactors (`GameplayStatics.GetAllActorsOfClass` "/Game/AI/NavPoint_BP.NavPoint_BP_C"))
    (for _array_element _outactors
      (set `NavPoint.bShowDebug` true _array_element)
      (`KismetSystemLibrary.PrintString` "NGraph"))))